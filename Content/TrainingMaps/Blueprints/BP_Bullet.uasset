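; BP_Bullet is a training-map projectile actor that flies forward when launched and removes itself after a short lifetime.
; Launch applies a velocity-change impulse to its Sphere component along the actor's forward vector.
; BeginPlay starts a delay that destroys the actor, and PrintYourName prints the actor's display name for debugging.
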(event EventBeginPlay
  (Utilities|FlowControl|Delay 1e+01)
  (Actor|DestroyActor))

(fn ConstructionScript)

(fn PrintYourName
  (Development|PrintString (Utilities|GetDisplayName self)))

(fn Launch
  (Physics|AddImpulse (Variables|Default|GetSphere) (* (Transformation|GetActorForwardVector) 4e+03) "None" true))